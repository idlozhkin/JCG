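; Card deck actor that builds, shuffles and deals the cards for the card game.
; CreateDeck clears the deck, constructs a card for every dignity and suit pair, mixes in a requested number of randomly picked trumps, then shuffles.
; Pop deals from the end of the array, first reshuffling the GameLogic discard pile back in when the deck is empty.
; AddCardAndShuffle returns a single card to the deck.
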(fn `AddCardAndShuffle`
  (params (Card :type "/Game/Development/Blueprints/Card/BP_BaseCard Object Reference"))
  (`KismetArrayLibrary.Array_Add` (`self.Cards`) Card)
  (`self.ShuffleDeck`))

(fn `AddCards`
  (bind _enumvalue (foreach `/Game/Development/Blueprints/Enums/E_Dignity` false)
    (:`LoopBody`
      (bind _enumvalue_2 (foreach `/Game/Development/Blueprints/Enums/E_Suit` false)
        (:`LoopBody`
          (bind _returnvalue (`|GenericCreateObject` "/Game/Development/Blueprints/Card/BP_Card.BP_Card_C"))
          (bind _card (`/Game/Development/Blueprints/Card/BP_Card.CreateCard` _returnvalue _enumvalue _enumvalue_2))
          (`KismetArrayLibrary.Array_Add` (`self.Cards`) _card))))))

(fn `AddTrumps`
  (params (Count :type Integer))
  (locals (Trumps :type "Array of /Game/Development/Blueprints/Card/BP_Trump Object Reference") (RandomTrump :type "/Game/Development/Blueprints/Card/BP_Trump Object Reference"))
  (bind _enumvalue (foreach `/Game/Development/Blueprints/Enums/E_Trump` false)
    (:`LoopBody`
      (bind _returnvalue (`|GenericCreateObject` "/Game/Development/Blueprints/Card/BP_Trump.BP_Trump_C"))
      (bind _card (`/Game/Development/Blueprints/Card/BP_Trump.CreateTrump` _returnvalue _enumvalue))
      (`KismetArrayLibrary.Array_Add` (`local.Trumps`) _card))
    (:`then`
      (for _ (range 1 (+ Count 1))
        (if (`KismetArrayLibrary.Array_IsNotEmpty` (`local.Trumps`))
          (bind _output_get (set `local.RandomTrump` (`KismetArrayLibrary.Array_Random` (`local.Trumps`))))
          (`KismetArrayLibrary.Array_Add` (`self.Cards`) _output_get)
          (`KismetArrayLibrary.Array_RemoveItem` (`local.Trumps`) _output_get)
          (`KismetSystemLibrary.PrintString` (`|GetEnumeratorNameAsString` (`/Game/Development/Blueprints/Card/BP_Trump.Trump` _output_get))))))))

(fn `ClearDeck`
  (`KismetArrayLibrary.Array_Clear` (`self.Cards`)))

(fn `CreateDeck`
  (params (TrumpsCount :type Integer))
  (`self.ClearDeck`)
  (`self.AddCards`)
  (`self.AddTrumps` TrumpsCount)
  (`self.ShuffleDeck`))

(fn `Pop`
  (returns (Card :type "/Game/Development/Blueprints/Card/BP_BaseCard Object Reference"))
  (locals (`-TempCard` :type "/Game/Development/Blueprints/Card/BP_BaseCard Object Reference"))
  (bind _cards (`self.Cards`))
  (bind _returnvalue (- (`KismetArrayLibrary.Array_Length` _cards) 1))
  (`|ExecutionSequence`
    (:`then_0`
      (if (`KismetArrayLibrary.Array_IsEmpty` (`self.Cards`))
        (`self.ShuffleDiscard` (`/Game/Development/Blueprints/BP_GameLogic.Discard` (`self.GameLogic`)))))
    (:`then_1`
      (bind _output_get (set `local.-TempCard` (`|GetArrayItem` _cards _returnvalue)))
      (`KismetArrayLibrary.Array_Remove` _cards _returnvalue)
      (return _output_get))))

(fn `ShuffleDeck`
  (`KismetArrayLibrary.Array_Shuffle` (`self.Cards`)))

(fn `ShuffleDiscard`
  (params (Discard :type "/Game/Development/Blueprints/BP_Discard Object Reference"))
  (for _array_element (`/Game/Development/Blueprints/BP_Discard.Discard` Discard)
    (`KismetArrayLibrary.Array_Add` (`self.Cards`) _array_element))
  (`/Game/Development/Blueprints/BP_Discard.ClearDiscard` (`local.Discard`))
  (`self.ShuffleDeck`))

(fn `UserConstructionScript`)
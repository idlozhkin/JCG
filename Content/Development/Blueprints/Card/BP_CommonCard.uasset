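; BP_CommonCard is a child card Blueprint representing a common card with a dignity (rank, spelled Diginity) and a suit.
; CreateCommonCard stores both values and returns the card itself, acting as a chainable initializer.
; GetStringCard overrides the parent version, prefixing the dignity enum name and a slash to the parent's string.
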(fn `CreateCommonCard`
  (params (Diginity :type "/Game/Development/Blueprints/Enums/E_Dignity Enum" :default "NewEnumerator0") (Suit :type "/Game/Development/Blueprints/Enums/E_Suit Enum" :default "NewEnumerator0"))
  (returns (CommonCard :type "/Game/Development/Blueprints/Card/BP_CommonCard Object Reference"))
  (set `self.Diginity` Diginity)
  (set `self.Suit` Suit)
  (return self))

(fn `GetStringCard`
  (returns (StringCard :type String))
  (bind _stringcard (`parent.GetStringCard`))
  (return (`KismetStringLibrary.Concat_StrStr` (`|GetEnumeratorNameAsString` (`self.Diginity`)) "/" _stringcard)))

(fn `UserConstructionScript`
  (`parent.UserConstructionScript`))
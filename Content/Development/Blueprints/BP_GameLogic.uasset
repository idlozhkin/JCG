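; Game manager for a two-player Blackjack-style card game to 21, with cyclic suit duels and trump cards.
; Spawns deck, discard, players and table widget, then handles draw, suit-choice, stop and trump actions.
; Suit comparisons decide which drawn cards are kept; a player finished at the aim can pick a suit that discards a matching opponent draw.
; Scores combine data-table values, trump bonuses and ace adjustment; when both turns end, it tallies the winner and restarts.
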(event `EventRestartGame`
  (`KismetSystemLibrary.Delay` 1.0)
  (`self.RestartGame`))

(event `self.ReceiveBeginPlay`
  (`self.InitGame`))

(fn `ChooseSuitClickButton`
  (params (Player :type "/Game/Development/Blueprints/BP_Player Object Reference") (Suit :type "/Game/Development/Blueprints/Enums/E_Suit Enum" :default "NewEnumerator0"))
  (if (`/Game/Development/Blueprints/BP_Player.CanChooseSuit` Player)
    (set `/Game/Development/Blueprints/BP_Player.CanChooseSuit` false Player)
    (set `/Game/Development/Blueprints/BP_Player.SuitChoosen` true Player)
    (`/Game/Development/Blueprints/BP_Player.ChooseSuit` Player Suit)
    (`self.TryCompare`)))

(fn `ChooseWinner`
  (returns (Outcome :type "/Game/Development/Blueprints/Enums/E_GameOutcome Enum"))
  (if (and (<= (`self.Score1`) (`self.Aim`)) (> (`self.Score2`) (`self.Aim`)))
    (return "NewEnumerator0")
    (elif (and (> (`self.Score1`) (`self.Aim`)) (<= (`self.Score2`) (`self.Aim`)))
      (return "NewEnumerator1")
      (elif (and (> (`self.Score1`) (`self.Aim`)) (> (`self.Score2`) (`self.Aim`)) (< (`self.Score1`) (`self.Score2`)))
        (return "NewEnumerator0")
        (elif (and (> (`self.Score1`) (`self.Aim`)) (> (`self.Score2`) (`self.Aim`)) (> (`self.Score1`) (`self.Score2`)))
          (return "NewEnumerator1")
          (elif (and (<= (`self.Score1`) (`self.Aim`)) (<= (`self.Score2`) (`self.Aim`)) (< (`self.Score1`) (`self.Score2`)))
            (return "NewEnumerator1")
            (elif (and (<= (`self.Score1`) (`self.Aim`)) (<= (`self.Score2`) (`self.Aim`)) (> (`self.Score1`) (`self.Score2`)))
              (return "NewEnumerator0")
              (else
                (return "NewEnumerator2")))))))))

(fn `CompareOneCard`
  (params (Player1Card :type Boolean))
  (bind _player2 (`self.Player2`))
  (bind _player1 (`self.Player1`))
  (if Player1Card
    (bind _compareresult (`self.SuitCompare` (`/Game/Development/Blueprints/Card/BP_Card.Suit` (`/Game/Development/Blueprints/BP_Player.Card` (`self.Player1`))) (`/Game/Development/Blueprints/BP_Player.Suit` (`self.Player2`))))
    (if (== _compareresult 0)
      (`/Game/Development/Blueprints/BP_Player.DiscardCardFromHand` (`self.Player1`))
      (set `/Game/Development/Blueprints/BP_Player.CanDraw` true (`self.Player1`))
      (else
        (`/Game/Development/Blueprints/BP_Player.AddCardToHand` (`self.Player1`))
        (bind _score (`self.CountScore` (`self.Player1`)))
        (bind _output_get (set `self.Score1` _score))
        (if (< _output_get (`self.Aim`))
          (set `/Game/Development/Blueprints/BP_Player.CanDraw` true (`self.Player1`))
          (else
            (set `/Game/Development/Blueprints/BP_Player.EndTurn` true (`self.Player1`))))))
    (set `/Game/Development/Blueprints/BP_Player.CanChooseSuit` true _player2)
    (set `/Game/Development/Blueprints/BP_Player.SuitChoosen` false _player2)
    (else
      (bind _compareresult_2 (`self.SuitCompare` (`/Game/Development/Blueprints/BP_Player.Suit` (`self.Player1`)) (`/Game/Development/Blueprints/Card/BP_Card.Suit` (`/Game/Development/Blueprints/BP_Player.Card` (`self.Player2`)))))
      (if (== _compareresult_2 0)
        (`/Game/Development/Blueprints/BP_Player.DiscardCardFromHand` (`self.Player2`))
        (set `/Game/Development/Blueprints/BP_Player.CanDraw` true (`self.Player2`))
        (else
          (`/Game/Development/Blueprints/BP_Player.AddCardToHand` (`self.Player2`))
          (bind _score_2 (`self.CountScore` (`self.Player2`)))
          (bind _output_get_2 (set `self.Score2` _score_2))
          (if (< _output_get_2 (`self.Aim`))
            (set `/Game/Development/Blueprints/BP_Player.CanDraw` true (`self.Player2`))
            (else
              (set `/Game/Development/Blueprints/BP_Player.EndTurn` true (`self.Player2`))))))
      (set `/Game/Development/Blueprints/BP_Player.CanChooseSuit` true _player1)
      (set `/Game/Development/Blueprints/BP_Player.SuitChoosen` false _player1))))

(fn `CompareTwoCards`
  (bind _player1 (`self.Player1`))
  (bind _player2 (`self.Player2`))
  (`|ExecutionSequence`
    (:`then_0`
      (bind _compareresult (`self.SuitCompare` (`/Game/Development/Blueprints/Card/BP_Card.Suit` (`/Game/Development/Blueprints/BP_Player.Card` (`self.Player1`))) (`/Game/Development/Blueprints/Card/BP_Card.Suit` (`/Game/Development/Blueprints/BP_Player.Card` (`self.Player2`)))))
      (if (== _compareresult -1)
        (`/Game/Development/Blueprints/BP_Player.AddCardToHand` (`self.Player1`))
        (`/Game/Development/Blueprints/BP_Player.DiscardCardFromHand` (`self.Player2`))
        (elif (== _compareresult 0)
          (`/Game/Development/Blueprints/BP_Player.AddCardToHand` (`self.Player1`))
          (`/Game/Development/Blueprints/BP_Player.AddCardToHand` (`self.Player2`))
          (else
            (`/Game/Development/Blueprints/BP_Player.DiscardCardFromHand` (`self.Player1`))
            (`/Game/Development/Blueprints/BP_Player.AddCardToHand` (`self.Player2`))))))
    (:`then_1`
      (bind _score (`self.CountScore` (`self.Player1`)))
      (set `self.Score1` _score)
      (bind _score_2 (`self.CountScore` (`self.Player2`)))
      (set `self.Score2` _score_2))
    (:`then_2`
      (if (< (`self.Score1`) (`self.Aim`))
        (set `/Game/Development/Blueprints/BP_Player.CanDraw` true (`self.Player1`))
        (else
          (set `/Game/Development/Blueprints/BP_Player.EndTurn` true (`self.Player1`))
          (set `/Game/Development/Blueprints/BP_Player.CanChooseSuit` true _player1)
          (set `/Game/Development/Blueprints/BP_Player.SuitChoosen` false _player1))))
    (:`then_3`
      (if (< (`self.Score2`) (`self.Aim`))
        (set `/Game/Development/Blueprints/BP_Player.CanDraw` true (`self.Player2`))
        (else
          (set `/Game/Development/Blueprints/BP_Player.EndTurn` true (`self.Player2`))
          (set `/Game/Development/Blueprints/BP_Player.CanChooseSuit` true _player2)
          (set `/Game/Development/Blueprints/BP_Player.SuitChoosen` false _player2))))))

(fn `CountScore`
  (params (Player :type "/Game/Development/Blueprints/BP_Player Object Reference"))
  (returns (Score :type Integer))
  (locals (Result :type Integer))
  (bind _diginitydatatable (`self.DiginityDataTable`))
  (set `local.Result` (+ (`local.Result`) (`/Game/Development/Blueprints/BP_Player.BonusScore` Player)))
  (for _array_element (`/Game/Development/Blueprints/BP_Player.Hand` Player)
    (bind _outrownames (`DataTableFunctionLibrary.GetDataTableRowNames` _diginitydatatable))
    (for _array_element_2 _outrownames
      (bind _returnvalue (`|GetDataTableRow` _diginitydatatable _array_element_2)
        (:`then`
          (bind (_name _value) (break `/Game/Development/Blueprints/Enums/S_Diginity` _returnvalue))
          (if (`|EnumEquality` _name (`/Game/Development/Blueprints/Card/BP_Card.Diginity` _array_element))
            (set `local.Result` (+ _value (`local.Result`))))))))
  (bind _recountscore (`self.RecountScoreWithAces` (`local.Player`) (`local.Result`)))
  (bind _output_get (set `local.Result` _recountscore))
  (return _output_get))

(fn `GetETrumpByText`
  (params (EnumText :type Text))
  (returns (Enum :type "/Game/Development/Blueprints/Enums/E_Trump Enum"))
  (bind _enumvalue (foreach `/Game/Development/Blueprints/Enums/E_Trump` false)
    (:`LoopBody`
      (if (`KismetTextLibrary.EqualEqual_TextText` (`KismetTextLibrary.Conv_StringToText` (`|GetEnumeratorNameAsString` _enumvalue)) EnumText)
        (return _enumvalue)))))

(fn `InitGame`
  (`|ExecutionSequence`
    (:`then_0`
      (set `self.Aim` 21)
      (set `self.TrumpCount` 3))
    (:`then_1`
      (bind _returnvalue (`|SpawnActorFromClass` "/Game/Development/Blueprints/BP_Deck.BP_Deck_C" (`KismetMathLibrary.MakeTransform` (0.0 0.0 0.0)) "Undefined" "OverrideRootScale" null null))
      (bind _output_get (set `self.Deck` _returnvalue))
      (set `/Game/Development/Blueprints/BP_Deck.GameLogic` self _output_get)
      (bind _returnvalue_2 (`|SpawnActorFromClass` "/Game/Development/Blueprints/BP_Discard.BP_Discard_C" (`KismetMathLibrary.MakeTransform` (0.0 0.0 0.0)) "Undefined" "OverrideRootScale" null null))
      (set `self.Discard` _returnvalue_2))
    (:`then_2`
      (bind _returnvalue_3 (`|SpawnActorFromClass` "/Game/Development/Blueprints/BP_Player.BP_Player_C" (`KismetMathLibrary.MakeTransform` (0.0 0.0 0.0)) "Undefined" "OverrideRootScale" null null))
      (bind _output_get_2 (set `self.Player1` _returnvalue_3))
      (set `/Game/Development/Blueprints/BP_Player.Discard` (`self.Discard`) _output_get_2)
      (bind _returnvalue_4 (`|SpawnActorFromClass` "/Game/Development/Blueprints/BP_Player.BP_Player_C" (`KismetMathLibrary.MakeTransform` (0.0 0.0 0.0)) "Undefined" "OverrideRootScale" null null))
      (bind _output_get_3 (set `self.Player2` _returnvalue_4))
      (set `/Game/Development/Blueprints/BP_Player.Discard` (`self.Discard`) _output_get_3))
    (:`then_3`
      (bind _returnvalue_5 (`|CreateWidget` "/Game/Development/Blueprints/Widgets/W_Table.W_Table_C"))
      (`UserWidget.AddToViewport` _returnvalue_5 0))
    (:`then_4`
      (`self.RestartGame`))))

(fn `PlusTwoTrump`
  (params (Player :type "/Game/Development/Blueprints/BP_Player Object Reference"))
  (`/Game/Development/Blueprints/BP_Player.AddBonusScore` Player 2))

(fn `RecountScoreWithAces`
  (params (Player :type "/Game/Development/Blueprints/BP_Player Object Reference") (Score :type Integer))
  (returns (RecountScore :type Integer))
  (locals (LocalScore :type Integer))
  (set `local.LocalScore` Score)
  (for _array_element (`/Game/Development/Blueprints/BP_Player.Hand` Player)
    (if (`|EnumEquality` (`/Game/Development/Blueprints/Card/BP_Card.Diginity` _array_element) "NewEnumerator12")
      (if (> (`local.LocalScore`) (`self.Aim`))
        (set `local.LocalScore` (- (`local.LocalScore`) 10)))))
  (return (`local.LocalScore`)))

(fn `RestartGame`
  (set `self.Score1` 0)
  (set `self.Score2` 0)
  (`/Game/Development/Blueprints/BP_Deck.CreateDeck` (`self.Deck`) (`self.TrumpCount`))
  (`/Game/Development/Blueprints/BP_Player.DiscardAllHand` (`self.Player1`))
  (`/Game/Development/Blueprints/BP_Player.DiscardAllHand` (`self.Player2`))
  (set `/Game/Development/Blueprints/BP_Player.CanDraw` true (`self.Player1`))
  (set `/Game/Development/Blueprints/BP_Player.CanDraw` true (`self.Player2`))
  (set `/Game/Development/Blueprints/BP_Player.EndTurn` false (`self.Player1`))
  (set `/Game/Development/Blueprints/BP_Player.EndTurn` false (`self.Player2`)))

(fn `StopClickButton`
  (params (Player :type "/Game/Development/Blueprints/BP_Player Object Reference"))
  (`/Game/Development/Blueprints/BP_Player.Stoped` Player)
  (`self.TryCompare`))

(fn `SuitCompare`
  (params (Suit1 :type "/Game/Development/Blueprints/Enums/E_Suit Enum" :default "NewEnumerator0") (Suit2 :type "/Game/Development/Blueprints/Enums/E_Suit Enum" :default "NewEnumerator0"))
  (returns (CompareResult :type Integer))
  (if (`|EnumEquality` Suit1 Suit2)
    (return 0)
    (elif (or (and (`|EnumEquality` (`local.Suit1`) "NewEnumerator0") (`|EnumEquality` (`local.Suit2`) "NewEnumerator2")) (and (`|EnumEquality` (`local.Suit1`) "NewEnumerator2") (`|EnumEquality` (`local.Suit2`) "NewEnumerator1")) (and (`|EnumEquality` (`local.Suit1`) "NewEnumerator1") (`|EnumEquality` (`local.Suit2`) "NewEnumerator0")))
      (return -1)
      (else
        (return 1)))))

(fn `TakeCard`
  (params (Player :type "/Game/Development/Blueprints/BP_Player Object Reference"))
  (locals (IsTrump :type Boolean :default true))
  (bind _card (`/Game/Development/Blueprints/BP_Player.Card` (`local.Player`)))
  (while (`local.IsTrump`)
    (bind _card_2 (`/Game/Development/Blueprints/BP_Deck.Pop` (`self.Deck`)))
    (bind _asbp_card (cast `/Game/Development/Blueprints/Card/BP_Card` _card_2)
      (:`then`
        (set `local.IsTrump` false)
        (set `/Game/Development/Blueprints/BP_Player.Card` _asbp_card (`local.Player`)))
      (:`CastFailed`
        (`/Game/Development/Blueprints/BP_Player.AddTrumpToHand` (`local.Player`) _card_2))))
  (bind _stringname (`/Game/Development/Blueprints/Card/BP_Card.GetStringName` _card))
  (`KismetSystemLibrary.PrintString` _stringname true true (struct :`G` 0.66 :`B` 1.0 :`A` 1.0) 3.0)
  (`/Game/Development/Blueprints/BP_Player.TakeCard` (`local.Player`) _card))

(fn `TakeCardClickButton`
  (params (Player :type "/Game/Development/Blueprints/BP_Player Object Reference"))
  (if (`/Game/Development/Blueprints/BP_Player.CanDraw` Player)
    (set `/Game/Development/Blueprints/BP_Player.CanDraw` false Player)
    (`self.TakeCard` Player)
    (`self.TryCompare`)))

(fn `TakeOpponent`
  (params (Player :type "/Game/Development/Blueprints/BP_Player Object Reference"))
  (returns (Opponent :type "/Game/Development/Blueprints/BP_Player Object Reference"))
  (if (== Player (`self.Player1`))
    (return (`self.Player2`))
    (else
      (return (`self.Player1`)))))

(fn `TryCompare`
  (bind _returnvalue (and (`KismetSystemLibrary.IsValid` (`/Game/Development/Blueprints/BP_Player.Card` (`self.Player1`))) (`/Game/Development/Blueprints/BP_Player.SuitChoosen` (`self.Player2`))))
  (`|ExecutionSequence`
    (:`then_0`
      (if (and (`KismetSystemLibrary.IsValid` (`/Game/Development/Blueprints/BP_Player.Card` (`self.Player1`))) (`KismetSystemLibrary.IsValid` (`/Game/Development/Blueprints/BP_Player.Card` (`self.Player2`))))
        (`self.CompareTwoCards`)
        (elif (or (and (`/Game/Development/Blueprints/BP_Player.SuitChoosen` (`self.Player1`)) (`KismetSystemLibrary.IsValid` (`/Game/Development/Blueprints/BP_Player.Card` (`self.Player2`)))) _returnvalue)
          (`self.CompareOneCard` _returnvalue))))
    (:`then_1`
      (if (and (`/Game/Development/Blueprints/BP_Player.EndTurn` (`self.Player1`)) (`/Game/Development/Blueprints/BP_Player.EndTurn` (`self.Player2`)))
        (set `/Game/Development/Blueprints/BP_Player.CanChooseSuit` false (`self.Player1`))
        (set `/Game/Development/Blueprints/BP_Player.CanChooseSuit` false (`self.Player2`))
        (`|ExecutionSequence`
          (:`then_0`
            (bind _outcome (`self.ChooseWinner`))
            (switch `/Game/Development/Blueprints/Enums/E_GameOutcome` _outcome
              (:`NewEnumerator0`
                (`/Engine/EditorBlueprintResources/StandardMacros.IncrementInt` (`self.WinningScore1`)))
              (:`NewEnumerator1`
                (`/Engine/EditorBlueprintResources/StandardMacros.IncrementInt` (`self.WinnigScore2`)))))
          (:`then_1`
            (`self.EventRestartGame`)))))))

(fn `UserConstructionScript`)

(fn `UseTrump`
  (params (Player :type "/Game/Development/Blueprints/BP_Player Object Reference") (TrumpText :type Text))
  (bind _enum (`self.GetETrumpByText` TrumpText))
  (`/Game/Development/Blueprints/BP_Player.DiscardTrump` Player _enum)
  (switch `/Game/Development/Blueprints/Enums/E_Trump` _enum
    (:`NewEnumerator0`
      (`self.PlusTwoTrump` (`local.Player`)))
    (:`NewEnumerator8`
      (`self.PlusTwoTrump` (`self.TakeOpponent` (`local.Player`))))))
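; BP_Player holds one player's state in a card game: hand, trump cards, chosen suit, score, bonus score, aim and turn or round state.
; A taken card is held as pending, then either added to the hand or sent to the Discard object.
; An active shield trump effect turns a discard into an add to hand, which clears the shield.
; Reinitializing sets a new aim, zeroes scores, discards the hand and resets the state.
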(fn `AddBonusScore`
  (params (Bonus :type Integer))
  (set `self.BonusScore` (+ Bonus (`self.BonusScore`))))

(fn `AddCardToHand`
  (`|ExecutionSequence`
    (:`then_0`
      (if (`self.ShieldTrumpEffect`)
        (set `self.ShieldTrumpEffect` false)))
    (:`then_1`
      (`KismetArrayLibrary.Array_Add` (`self.Hand`) (`self.Card`))
      (set `self.Card` null))))

(fn `AddTrumpToHand`
  (params (Card :type "/Game/Development/Blueprints/Card/BP_BaseCard Object Reference"))
  (bind _asbp_trump (cast `/Game/Development/Blueprints/Card/BP_Trump` Card))
  (`KismetArrayLibrary.Array_Add` (`self.Trumps`) _asbp_trump))

(fn `ChooseSuit`
  (params (Suit :type "/Game/Development/Blueprints/Enums/E_Suit Enum" :default "NewEnumerator0"))
  (set `self.Suit` Suit))

(fn `DiscardAllHand`
  (for _array_element (`self.Hand`)
    (`/Game/Development/Blueprints/BP_Discard.DiscardCard` (`self.Discard`) _array_element))
  (`KismetArrayLibrary.Array_Clear` (`self.Hand`)))

(fn `DiscardCardFromHand`
  (if (`self.ShieldTrumpEffect`)
    (`self.AddCardToHand`)
    (else
      (`/Game/Development/Blueprints/BP_Discard.DiscardCard` (`self.Discard`) (`self.Card`))
      (set `self.Card` null))))

(fn `DiscardTrump`
  (params (Trump :type "/Game/Development/Blueprints/Enums/E_Trump Enum" :default "NewEnumerator0"))
  (for _array_element (`self.Trumps`)
    (if (`|EnumEquality` (`/Game/Development/Blueprints/Card/BP_Trump.Trump` _array_element) Trump)
      (`KismetArrayLibrary.Array_RemoveItem` (`self.Trumps`) _array_element))))

(fn `ReinitVars`
  (params (Aim :type Integer))
  (`|ExecutionSequence`
    (:`then_0`
      (set `self.Aim` Aim)
      (set `self.Score` 0)
      (set `self.BonusScore` 0))
    (:`then_2`
      (`self.DiscardAllHand`))
    (:`then_3`
      (set `self.State` "NewEnumerator2"))))

(fn `TakeCard`
  (params (Card :type "/Game/Development/Blueprints/Card/BP_Card Object Reference"))
  (returns (ResCard :type "/Game/Development/Blueprints/Card/BP_Card Object Reference"))
  (bind _output_get (set `self.Card` Card))
  (return _output_get))

(fn `Taken`
  (if (`|EnumEquality` (`self.State`) "NewEnumerator2")
    (set `self.State` "NewEnumerator3")))

(fn `UserConstructionScript`)